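; BP_GameInGameHostSlider is an actor that slides back and forth along the world X axis around its starting location.
; BeginPlay stores that home location, and Tick advances an offset at fixed speed, reversing direction when the next step would cross either symmetric limit.
; The actor is moved without sweep, one extra step ahead of the stored offset because the step is added again after updating.
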(event EventBeginPlay
  (Variables|Default|SetHomeLocation (Transformation|GetActorLocation))
  (Variables|Default|SetDir 1.0)
  (Variables|Default|SetOffset 0.0))

(event Collision|EventActorBeginOverlap
  (params (OtherActor :type Actor%20Object%20Reference)))

(event EventTick
  (params (DeltaSeconds :type Float%20%28single-precision%29))
  (bind _homelocation (Variables|Default|GetHomeLocation))
  (if (> (+ (Variables|Default|GetOffset) (* (* (Variables|Default|GetDir) (Math|Float|MakeLiteralFloat 4.2e+02)) DeltaSeconds)) (Math|Float|MakeLiteralFloat 6.5e+02))
    (Variables|Default|SetDir -1.0)
    (elif (< (+ (Variables|Default|GetOffset) (* (* (Variables|Default|GetDir) (Math|Float|MakeLiteralFloat 4.2e+02)) DeltaSeconds)) (Math|Float|MakeLiteralFloat -6.5e+02))
      (Variables|Default|SetDir 1.0)))
  (Variables|Default|SetOffset (+ (Variables|Default|GetOffset) (* (* (Variables|Default|GetDir) (Math|Float|MakeLiteralFloat 4.2e+02)) DeltaSeconds)))
  (Transformation|SetActorLocation (Math|Vector|MakeVector (+ (.X (Math|Vector|BreakVector _homelocation)) (+ (Variables|Default|GetOffset) (* (* (Variables|Default|GetDir) (Math|Float|MakeLiteralFloat 4.2e+02)) DeltaSeconds))) (.Y (Math|Vector|BreakVector _homelocation)) (.Z (Math|Vector|BreakVector _homelocation))) false false))

(fn ConstructionScript)